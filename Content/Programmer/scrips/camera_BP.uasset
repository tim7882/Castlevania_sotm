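; A zone camera actor that follows the player along Y and Z within set bounds while keeping its X position fixed.
; Every tick the camera moves to the player's location, clamped to the world bounds of CameraBoundBox.
; When a MyCharactor overlaps ActorCollisionbox, the player's view blends to this actor using configurable blend settings.
; The construction script applies variable-driven transforms and extents to the camera and both boxes.
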(event OnComponentBeginOverlap(ActorCollisionbox)
  (params (OverlappedComponent :type Primitive%20Component%20Object%20Reference) (OtherActor :type Actor%20Object%20Reference) (OtherComp :type Primitive%20Component%20Object%20Reference) (OtherBodyIndex :type Integer) (bFromSweep :type Boolean) (SweepResult :type Hit%20Result%20Structure%20%28by%20ref%29))
  (Utilities|Casting|CastToMyCharactor OtherActor)
  (Game|Player|SetViewTargetwithBlend (Game|GetPlayerController 0) self (Variables|CameraView|GetBlendTime) (Variables|CameraView|GetBlendFunc) (Variables|CameraView|GetBlendExp) false))

(event EventBeginPlay)

(event EventTick
  (params (DeltaSeconds :type Float%20%28single-precision%29))
  (bind _returnvalue (Game|GetPlayerCharacter 0))
  (bind _cameraboundbox (Variables|Default|GetCameraBoundBox))
  (bind _returnvalue_2 (Transformation|GetActorLocation _returnvalue))
  (bind (_origin _boxextent) (Collision|GetComponentBounds _cameraboundbox))
  (bind _returnvalue_3 (- _origin _boxextent))
  (bind _returnvalue_4 (+ _origin _boxextent))
  (Transformation|SetWorldLocation (Variables|Default|GetCamera) (Math|Vector|MakeVector (.x (Transformation|GetWorldLocation (Variables|Default|GetCamera))) (Math|Float|Clamp(Float) (.y _returnvalue_2) (.y _returnvalue_3) (.y _returnvalue_4)) (Math|Float|Clamp(Float) (.z _returnvalue_2) (.z _returnvalue_3) (.z _returnvalue_4))) false false))

(fn ConstructionScript
  (bind _cameraboundbox (Variables|Default|GetCameraBoundBox))
  (bind _actorcollisionbox (Variables|Default|GetActorCollisionbox))
  (Utilities|FlowControl|Sequence
    (:then_0
      (Transformation|SetRelativeTransform (Variables|Default|GetCamera) (Variables|Default|GetCameraTransform) false false))
    (:then_1
      (Transformation|SetRelativeTransform _actorcollisionbox (Variables|Default|GetActorCollisionTransform) false false)
      (Components|Box|SetBoxExtent _actorcollisionbox (Variables|Default|GetActorCollisionExtent) true))
    (:then_2
      (Transformation|SetRelativeTransform _cameraboundbox (Variables|Default|GetCameraBoxTransform) false false)
      (Components|Box|SetBoxExtent _cameraboundbox (Variables|Default|GetCameraBoxExtent) true))))