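; Bullet actor that stands in for the player's knife, clearing the player's HasKnife flag while it exists.
; On BeginPlay it caches the player pawn as MyCharactor and starts a six-second timeout.
; The timeout, or a Box overlap with the player, leads to shared cleanup that restores HasKnife and destroys the actor.
; Overlaps with other actors do nothing, and the graphs contain no movement or damage logic.
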(event OnComponentBeginOverlap(Box)
  (params (OverlappedComponent :type Primitive%20Component%20Object%20Reference) (OtherActor :type Actor%20Object%20Reference) (OtherComp :type Primitive%20Component%20Object%20Reference) (OtherBodyIndex :type Integer) (bFromSweep :type Boolean) (SweepResult :type Hit%20Result%20Structure%20%28by%20ref%29))
  ;[1 1 1] Deletion Code
  (if (not (!= OtherActor (Variables|Default|GetPlayerObject)))
    (Variables|/Game/Programmer/scrips/MyCharactor.MyCharactor_C|SethasKnife (Variables|Default|GetPlayerObject) true)
    (Actor|DestroyActor)))

(event EventBeginPlay
  ;[1 1 1] BulletBeginning
  (bind _asmy_charactor (Utilities|Casting|CastToMyCharactor (Game|Player|GetPlayerPawn 0)))
  (bind _output_get (Variables|Default|SetPlayerObject _asmy_charactor))
  (Variables|/Game/Programmer/scrips/MyCharactor.MyCharactor_C|SethasKnife _output_get false)
  (Utilities|FlowControl|Delay 6.0)
  ;[1 1 1] Deletion Code
  (Variables|/Game/Programmer/scrips/MyCharactor.MyCharactor_C|SethasKnife (Variables|Default|GetPlayerObject) true)
  (Actor|DestroyActor))

(fn ConstructionScript)