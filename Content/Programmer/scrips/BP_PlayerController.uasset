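; Player controller for a sidescroller that handles the player's death sequence.
; Its onDeath event unpossesses the pawn, fades the camera out and holds it, and shows the WBP_YouDied widget.
; After a short delay it removes the widget and calls RestartGame on the sidescroller game mode.
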(event Custom|onDeath
  (Pawn|UnPossess)
  (CameraFades|StartCameraFade :self (Variables|Default|GetPlayerCameraManager) :ToAlpha 1.0 :Duration 2.0 :bHoldWhenFinished true)
  (bind _returnvalue (UserInterface|CreateWidget "/Game/Designer/HUD/UI/WBP_YouDied.WBP_YouDied_C" self))
  (UserInterface|Viewport|AddtoViewport _returnvalue 0)
  (Utilities|FlowControl|Delay 5.0)
  (Widget|RemovefromParent _returnvalue)
  (bind _assidescroller_gamemode (Utilities|Casting|CastTosidescroller_gamemode (Game|GetGameMode)))
  (Class|GameMode|RestartGame _assidescroller_gamemode))

(event EventBeginPlay)

(event EventTick
  (params (DeltaSeconds :type Float%20%28single-precision%29)))

(fn ConstructionScript)